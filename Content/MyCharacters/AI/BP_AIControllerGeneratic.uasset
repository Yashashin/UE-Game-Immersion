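; AI controller Blueprint that runs the BT_AI behavior tree and turns perception events into blackboard data.
; Each perception update is passed to sight and hearing handlers, which filter by stimulus sense class.
; Sight sets TargetActor when an actor is sensed and clears it when sight is lost.
; Hearing writes the stimulus position to Investigate Location and shows the controlled BP_AI pawn's investigate widget.
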(event OnTargetPerceptionUpdated(AIPerception)
  (params (Actor :type Actor%20Object%20Reference) (Stimulus :type AI%20Stimulus%20Structure))
  ;[0.02315 0.0356 0.05286] Detect/Chase Target
  (CallFunction|SightDetection Actor Stimulus)
  (CallFunction|HearingDetection Actor Stimulus))

(event EventBeginPlay
  (AI|RunBehaviorTree "/Game/MyCharacters/AI/BT_AI.BT_AI"))

(event EventTick
  (params (DeltaSeconds :type Float%20%28single-precision%29)))

(fn ConstructionScript)

(fn SightDetection
  (params (Actor :type Actor%20Object%20Reference) (Stimulus :type AI%20Stimulus%20Structure))
  (bind _returnvalue (Class|AIPerceptionSystem|GetSenseClassforStimulus Stimulus))
  (if (== _returnvalue "/Script/AIModule.AISense_Sight")
    (if (.bSuccessfullySensed (Utilities|Struct|BreakAIStimulus Stimulus))
      (AI|Components|Blackboard|SetValueasObject (AI|GetBlackboard 0) (Utilities|Name|MakeLiteralName "TargetActor") Actor)
      (else
        (AI|Components|Blackboard|SetValueasObject (AI|GetBlackboard 0) (Utilities|Name|MakeLiteralName "TargetActor") 0)))))

(fn HearingDetection
  (params (Actor :type Actor%20Object%20Reference) (Stimulus :type AI%20Stimulus%20Structure))
  (bind _returnvalue (Class|AIPerceptionSystem|GetSenseClassforStimulus Stimulus))
  (if (== _returnvalue "/Script/AIModule.AISense_Hearing")
    (AI|Components|Blackboard|SetValueasVector (AI|GetBlackboard 0) (Utilities|Name|MakeLiteralName "Investigate Location") (.StimulusLocation (Utilities|Struct|BreakAIStimulus Stimulus)))
    (bind _asbp_ai (Utilities|Casting|CastToBP_AI (Pawn|GetControlledPawn)))
    (Class|MyGameAI|SetInvestigateWidgetVisible _asbp_ai)))