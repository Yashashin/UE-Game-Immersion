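; BP_Dummy is a test dummy character that reacts to damage and can collapse into a ragdoll.
; Any damage prints a debug message and plays a random hit montage from the HitAnim array.
; The RagDoll event turns on mesh physics simulation after a short delay, with no caller in this graph.
; Unconnected leftover nodes for toggling an assassination widget and launching the character forward never run.
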(event Custom|RagDoll
  (Utilities|FlowControl|Delay 1.9)
  (Physics|SetSimulatePhysics (Variables|Character|GetMesh) true))

(event EventBeginPlay)

(event Collision|EventActorBeginOverlap
  (params (OtherActor :type Actor%20Object%20Reference)))

(event EventTick
  (params (DeltaSeconds :type Float%20%28single-precision%29)))

(event Game|Damage|EventAnyDamage
  (params (Damage :type Float%20%28single-precision%29) (DamageType :type Damage%20Type%20Object%20Reference) (InstigatedBy :type Controller%20Object%20Reference) (DamageCauser :type Actor%20Object%20Reference))
  (Development|PrintString "Damage!!!")
  (Animation|PlayAnimMontage (Utilities|Array|Get(acopy) (Variables|Default|GethitAnim) (Math|Random|RandomIntegerinRange 0 (- (Utilities|Array|Length (Variables|Default|GethitAnim)) 1))) 1.0 "None"))

(fn ConstructionScript)